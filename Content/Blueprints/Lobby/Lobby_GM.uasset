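; Lobby game mode that tracks connected lobby player controllers and keeps the lobby player count up to date.
; On login it adds the Lobby_PC to AllPC, waits briefly, then has that controller run HUDLobby.
; Both login and logout pass the new AllPC length to Lobby_GS through UpdatePlayers.
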(event `self.K2_PostLogin`
  (params (NewPlayer :type "PlayerController Object Reference"))
  (bind _aslobby_pc (cast `/Game/Blueprints/Lobby/Lobby_PC` NewPlayer))
  (`KismetArrayLibrary.Array_Add` (`self.AllPC`) _aslobby_pc)
  (`KismetSystemLibrary.Delay` 0.1)
  (`/Game/Blueprints/Lobby/Lobby_PC.HUD - Lobby` _aslobby_pc)
  (bind _aslobby_gs (cast `/Game/Blueprints/Lobby/Lobby_GS` (`GameplayStatics.GetGameState`)))
  (`/Game/Blueprints/Lobby/Lobby_GS.UpdatePlayers` _aslobby_gs (`KismetArrayLibrary.Array_Length` (`self.AllPC`))))

(event `self.K2_OnLogout`
  (params (ExitingController :type "Controller Object Reference"))
  (bind _aslobby_pc (cast `/Game/Blueprints/Lobby/Lobby_PC` ExitingController))
  (`KismetArrayLibrary.Array_RemoveItem` (`self.AllPC`) _aslobby_pc)
  (bind _aslobby_gs (cast `/Game/Blueprints/Lobby/Lobby_GS` (`GameplayStatics.GetGameState`)))
  (`/Game/Blueprints/Lobby/Lobby_GS.UpdatePlayers` _aslobby_gs (`KismetArrayLibrary.Array_Length` (`self.AllPC`))))

(fn `UserConstructionScript`)