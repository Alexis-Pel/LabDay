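; Main menu PlayerController that creates the menu widget and handles online session hosting, searching and joining.
; BeginPlay shows the cursor in Game and UI mode and builds HUD_Menu only on the Remote authority branch; the U key creates it directly, bypassing both checks.
; Hosting opens Lobby as a listen server, and searching fills SessionsBox with HUD_Session entries.
; Joining uses a search result or an "open" console command with an IP.
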(event `self.ReceiveBeginPlay`
  ;[0.3768 0.4445 0] Init
  (`self.HUD - Menu`)
  (`self.Init Cursor`))

(event `HUD - Menu`
  ;[0.5991 0 0.2249] HUD Menu
  (`/Engine/EditorBlueprintResources/ActorMacros.Switch Has Authority`
    (:`Remote`
      (`/Engine/EditorBlueprintResources/StandardMacros.IsValid` (`self.HUD_Menu`)
        (:`Is Not Valid`
          (bind _returnvalue (`|CreateWidget` "/Game/HUD/Menu/HUD_Menu.HUD_Menu_C" :!label _label))
          (bind _output_get (set `self.HUD_Menu` _returnvalue))
          (`UserWidget.AddToViewport` _output_get 0))))))

(event `Init Cursor`
  ;[0.5314 0 0.2933] Init Cursor
  (set `self.bShowMouseCursor` true)
  (`WidgetBlueprintLibrary.SetInputMode_GameAndUIEx` self null "LockAlways" false))

(event `Key|U`
  (params (Key :type "Key Structure"))
  ;[0.5991 0 0.2249] HUD Menu
  (:`Pressed`
    (goto _label)))

(event `Heberger`
  ;[0 0.8116 0.009662] Héberger
  (`CreateSessionCallbackProxy.CreateSession` self 4
    (:`OnSuccess`
      (`GameplayStatics.OpenLevel` "Lobby" true "listen"))))

(event `Rejoindre`
  (params (IP :type String))
  ;[0 0.04831 0.773] Rejoindre
  (`KismetSystemLibrary.ExecuteConsoleCommand` (`KismetStringLibrary.Concat_StrStr` "open " IP) null))

(event `Rechercher`
  (`PanelWidget.ClearChildren` (`/Game/HUD/Menu/HUD_Menu.SessionsBox` (`self.HUD_Menu`)))
  (set `self.IsFindingSessions` true)
  (bind _results (`FindSessionsCallbackProxy.FindSessions` self 4)
    (:`OnSuccess`
      (for _array_element _results
        (bind _returnvalue (`|CreateWidget` "/Game/HUD/HUD_Session.HUD_Session_C" null _array_element))
        (`PanelWidget.AddChild` (`/Game/HUD/Menu/HUD_Menu.SessionsBox` (`self.HUD_Menu`)) _returnvalue))
      (set `self.IsFindingSessions` false))))

(event `JoinSession`
  (params (SearchResult :type "BlueprintSessionResult Structure (by ref)"))
  (`JoinSessionCallbackProxy.JoinSession` self SearchResult))

(fn `UserConstructionScript`)